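; Actor component for inventory persistence, holding inventory data in InventSave and moving it to and from save games.
; SaveInventory copies InventSave into the save object held by InvGameInstance and writes it to the "InventorySave" slot.
; LoadInventory restores InventSave from a SaveInventory object, but reads from an empty slot name rather than "InventorySave".
; FindItemSlot is an empty stub, and the event graph has no active logic.
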(fn `FindItemSlot`)

(fn `LoadInventory`
  (bind _returnvalue (`GameplayStatics.LoadGameFromSlot` ""))
  (bind _assave_inventory (cast `/Game/HSB/BluePrints/SaveInventory` _returnvalue))
  (set `self.InventSave` (`/Game/HSB/BluePrints/SaveInventory.Inventory` _assave_inventory)))

(fn `SaveInventory`
  (bind _asinv_game_instance (cast `/Game/HSB/BluePrints/InvGameInstance` (`GameplayStatics.GetGameInstance`)))
  (bind _as_save_data (`/Game/HSB/BluePrints/InvGameInstance.As Save Data` _asinv_game_instance))
  (set `/Game/HSB/BluePrints/SaveInventory.Inventory` (`self.InventSave`) _as_save_data)
  (`GameplayStatics.SaveGameToSlot` _as_save_data "InventorySave"))