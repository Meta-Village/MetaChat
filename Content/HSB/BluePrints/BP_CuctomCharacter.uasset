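; BP_CuctomCharacter is a modular character preview for character customization.
; The construction script makes the hair, head, upper body, lower body and feet meshes follow the main Mesh's pose through leader pose.
; On BeginPlay it adds the WBP_CharacterCustom_Main widget to the viewport and restricts its SceneCaptureComponent2D to showing only this actor's components.
; A slow mesh rotation exists but is disconnected.
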(event `self.ReceiveBeginPlay`
  (`|ExecutionSequence`
    (:`then_0`
      (bind _returnvalue (`|CreateWidget` "/Game/HSB/UI/WBP_CharacterCustom_Main.WBP_CharacterCustom_Main_C" (`GameplayStatics.GetPlayerController` 0)))
      (`UserWidget.AddToViewport` _returnvalue 0)
      (`SceneCaptureComponent.ShowOnlyActorComponents` (`self.SceneCaptureComponent2D`) self false))))

(event `self.ReceiveTick`
  (params (DeltaSeconds :type "Float (single-precision)")))

(fn `UserConstructionScript`
  (`SkinnedMeshComponent.SetLeaderPoseComponent` (`self.HairMesh`) (`self.Mesh`) false false)
  (`SkinnedMeshComponent.SetLeaderPoseComponent` (`self.HeadMesh`) (`self.Mesh`) false false)
  (`SkinnedMeshComponent.SetLeaderPoseComponent` (`self.LowerBodyMesh`) (`self.Mesh`) false false)
  (`SkinnedMeshComponent.SetLeaderPoseComponent` (`self.UpperBodyMesh`) (`self.Mesh`) false false)
  (`SkinnedMeshComponent.SetLeaderPoseComponent` (`self.FeetMesh`) (`self.Mesh`) false false))