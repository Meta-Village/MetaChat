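; Modular customizable player character with push-to-talk voice chat.
; Head, feet, hair and body meshes follow the main mesh via leader pose, and BeginPlay calls Load and removes PointLightCustom in the PrototypeMain level.
; BeginPlay also creates a VOIPTalker, retries until PlayerState is valid to register it, and enables loopback when locally controlled.
; Holding V toggles speaking through console commands and shows a sound icon widget.
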(event `self.ReceiveBeginPlay`
  (`|ExecutionSequence`
    (:`then_0`
      ;[1 1 1] SubmitcustomizationData(),
      ; UpdateCharacterAppearance() 같이 실행됨
      (`self.Load`))
    (:`then_1`
      (bind _returnvalue (`AddComponent|NODE_AddVOIPTalker-0`))
      (bind _output_get (set `self.VOIP_REF` _returnvalue))
      (`/Engine/EditorBlueprintResources/StandardMacros.IsValid` (`self.PlayerState`) :!label _label
        (:`Is Valid`
          (`VOIPTalker.RegisterWithPlayerState` _output_get (`self.PlayerState`))
          (`VOIPStatics.SetMicThreshold` -1.0)
          (set `VOIPTalker.Settings` (make `VoiceSettings` (`self.CapsuleComponent`)) (`self.VOIP_REF`))
          (if (`self.IsLocallyControlled`)
            (`KismetSystemLibrary.ExecuteConsoleCommand` "OSS.VoiceLoopback 1" null)))
        (:`Is Not Valid`
          (`KismetSystemLibrary.Delay` 0.2)
          (goto _label))))
    (:`then_2`
      (bind _returnvalue_2 (`GameplayStatics.GetCurrentLevelName` true))
      (if (`KismetStringLibrary.EqualEqual_StrStr` _returnvalue_2 "PrototypeMain")
        (`ActorComponent.K2_DestroyComponent` (`self.PointLight (Custom)`))))))

(event `self.ReceiveTick`
  (params (DeltaSeconds :type "Float (single-precision)")))

(event `Key|V`
  (params (Key :type "Key Structure"))
  (:`Pressed`
    (`KismetSystemLibrary.ExecuteConsoleCommand` "ToggleSpeaking 1" null)
    (bind _returnvalue (`|CreateWidget` "/Game/XR_YWK/UI/WB_SoundIcon.WB_SoundIcon_C"))
    (bind _output_get (set `self.Sound Widget` _returnvalue))
    (`UserWidget.AddToViewport` _output_get 0))
  (:`Released`
    (`KismetSystemLibrary.ExecuteConsoleCommand` "ToggleSpeaking 0" null)
    (`Widget.RemoveFromParent` (`self.Sound Widget`))))

(fn `UserConstructionScript`
  (`SkinnedMeshComponent.SetLeaderPoseComponent` (`self.HeadMeshComp`) (`self.Mesh`) false false)
  (`SkinnedMeshComponent.SetLeaderPoseComponent` (`self.FeetMeshComp`) (`self.Mesh`) false false)
  (`SkinnedMeshComponent.SetLeaderPoseComponent` (`self.HairMeshComp`) (`self.Mesh`) false false)
  (`SkinnedMeshComponent.SetLeaderPoseComponent` (`self.UpperBodyMeshComp`) (`self.Mesh`) false false)
  (`SkinnedMeshComponent.SetLeaderPoseComponent` (`self.LowerBodyMeshComp`) (`self.Mesh`) false false))