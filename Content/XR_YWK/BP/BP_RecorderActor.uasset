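; BP_RecorderActor is an actor that records audio from the Recording submix, controlled by an on-screen record button widget.
; On BeginPlay it adds WB_RecordButton to the first player's viewport and binds the widget's start and stop events.
; Start begins submix output recording; stop exports a WAV named "test" to a hardcoded local project folder.
; Both handlers print debug messages to screen.
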(event `self.ReceiveBeginPlay`
  (if (not false)
    (bind _returnvalue (`|CreateWidget` "/Game/XR_YWK/UI/WB_RecordButton.WB_RecordButton_C" (`GameplayStatics.GetPlayerController` 0)))
    (bind _output_get (set `self.Target` _returnvalue))
    (`UserWidget.AddToViewport` _output_get 0)
    (`|ExecutionSequence`
      (:`then_0`
        (add `/Game/XR_YWK/UI/WB_RecordButton.StartRecording` _output_get (delegate `StartRecording`)))
      (:`then_1`
        (add `/Game/XR_YWK/UI/WB_RecordButton.StopRecording` _output_get (delegate `StopRecording`))))))

(event `StartRecording`
  (`KismetSystemLibrary.PrintString` "녹음 시작")
  (`AudioMixerBlueprintLibrary.StartRecordingOutput` 0.0 "/Game/XR_YWK/Recording.Recording")
  (`KismetSystemLibrary.PrintString` "Start" true true (struct :`G` 0.66 :`B` 1.0 :`A` 1.0) 3.0 "-1"))

(event `StopRecording`
  (`KismetSystemLibrary.PrintString` "녹음 끝")
  (`AudioMixerBlueprintLibrary.StopRecordingOutput` "WavFile" "test" "C:\\project\\MetaChat\\savewave" "/Game/XR_YWK/Recording.Recording" null)
  (`KismetSystemLibrary.PrintString` "stop" true true (struct :`G` 0.66 :`B` 1.0 :`A` 1.0) 2.0 "1"))

(fn `UserConstructionScript`)