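; Screen actor that receives another user's shared screen as a Pixel Streaming viewer over a hardcoded WebSocket signalling server.
; Begin, Stop and Change functions control the connection and subscription, and connecting triggers a streamer list fetch.
; That list is filtered to sharing users, then it subscribes to the chosen or default stream, disconnecting if none are sharing and it isn't watching.
; Signalling and peer component events relay config, offer/answer and ICE candidates for the WebRTC handshake.
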(event `self.ReceiveBeginPlay`)

(event `GetStreamerIDList`
  (bind _viewsharinguserstreamid (`self.ViewSharingUserStreamID`))
  (bind _viewsharinguserstreamid_2 (`self.ViewSharingUserStreamID`))
  (bind _streamerlist (`AsyncAction_GetStreamers.GetStreamerIdList` (`self.PixelStreamingSignalling`) :!label _label)
    (:`Completed`
      (bind _returnvalue (`self.GetSharingUsers` _streamerlist))
      (if (`KismetStringLibrary.IsEmpty` _returnvalue)
        (bind _returnvalue_2 (`self.GetLookStreaming`))
        (if _returnvalue_2
          (if (not (`KismetStringLibrary.IsEmpty` _viewsharinguserstreamid))
            (`PixelStreamingSignallingComponent.Subscribe` (`self.PixelStreamingSignalling`) _viewsharinguserstreamid))
          (else
            (`PixelStreamingSignallingComponent.Disconnect` (`self.PixelStreamingSignalling`))))
        (elif (`KismetStringLibrary.IsEmpty` _viewsharinguserstreamid_2)
          (`PixelStreamingSignallingComponent.Subscribe` (`self.PixelStreamingSignalling`) _returnvalue)
          (else
            (`PixelStreamingSignallingComponent.Subscribe` (`self.PixelStreamingSignalling`) _viewsharinguserstreamid_2)))))))

(event `self.PixelStreamingSignalling.OnConnected`
  (set `self.IsConnected` true)
  (goto _label))

(event `self.PixelStreamingSignalling.OnConfig`
  (params (Config :type "PixelStreamingRTCConfigWrapper Structure"))
  (`PixelStreamingPeerComponent.SetConfig` (`self.PixelStreamingPeer`) Config))

(event `self.PixelStreamingSignalling.OnOffer`
  (params (Offer :type String))
  (bind _returnvalue (`PixelStreamingPeerComponent.CreateAnswer` (`self.PixelStreamingPeer`) Offer))
  (`PixelStreamingSignallingComponent.SendAnswer` (`self.PixelStreamingSignalling`) _returnvalue))

(event `self.PixelStreamingSignalling.OnIceCandidate`
  (params (Candidate :type "PixelStreamingIceCandidateWrapper Structure"))
  (`PixelStreamingPeerComponent.ReceiveIceCandidate` (`self.PixelStreamingPeer`) Candidate))

(event `self.PixelStreamingPeer.OnIceCandidate`
  (params (Candidate :type "PixelStreamingIceCandidateWrapper Structure"))
  (`PixelStreamingSignallingComponent.SendIceCandidate` (`self.PixelStreamingSignalling`) Candidate))

(event `self.PixelStreamingSignalling.OnAnswer`
  (params (Answer :type String))
  (`KismetSystemLibrary.PrintString` "ANswer" true true (struct :`G` 0.66 :`B` 1.0 :`A` 1.0) 10.0))

(fn `BeginLookPixelStreaming`
  (if (`self.IsConnected`)
    (`self.GetStreamerIDList`)
    (else
      (`PixelStreamingSignallingComponent.Connect` (`self.PixelStreamingSignalling`) "ws://master-of-prediction.shop:8124"))))

(fn `ChangeLookPixelStreaming`
  (bind _pixelstreamingsignalling (`self.PixelStreamingSignalling`))
  (`PixelStreamingSignallingComponent.Unsubscribe` _pixelstreamingsignalling)
  (`PixelStreamingSignallingComponent.Subscribe` _pixelstreamingsignalling (`self.ViewSharingUserStreamID`)))

(fn `ConnectPixelStreaming`
  (`PixelStreamingSignallingComponent.Connect` (`self.PixelStreamingSignalling`) "ws://master-of-prediction.shop:8124"))

(fn `StopLookPixelStreaming`
  (if (`self.IsConnected`)
    (`PixelStreamingSignallingComponent.Disconnect` (`self.PixelStreamingSignalling`))
    (set `self.IsConnected` false)))

(fn `UserConstructionScript`)